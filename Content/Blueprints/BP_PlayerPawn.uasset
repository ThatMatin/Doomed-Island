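; Player pawn that drives foot IK on the hero AnimBlueprint, plus local HUD widgets, zoom and debug keys for slow motion and IK tuning.
; Each tick, foot traces feed interpolated foot offsets, rotations, hip drop and capsule height when stationary, resetting during movement.
; An optional optimization gates IK updates off once feet settle, reopening on movement or turning.
; An Adpation_2 graph for slope-aligning the mesh is not called from Tick.
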(event EventTick
  (params (DeltaSeconds :type Float%20%28single-precision%29))
  (Utilities|FlowControl|Sequence
    (:then_0
      (if (Pawn|IsLocallyControlled)
        (Development|PrintString (Utilities|String|ToString(Float) (Variables|/Script/CoopGame.SHealthComponent|GetHealth (Variables|Default|GetHealthComp))) true true "(R=0.000000,G=0.660000,B=1.000000,A=1.000000)" 0.0)))
    (:then_1
      (Variables|Default|SetDeltaSeconds DeltaSeconds)
      ;[1 1 1] IK Node
      (Utilities|FlowControl|Sequence
        (:then_0
          (|IkGrap_2))))))

(event EventBeginPlay
  (Utilities|FlowControl|Sequence
    (:then_0
      ;[1 1 1] Creating a refference to our Anim Instance at Begin Play
      (bind _asue4asp_hero_tpp_anim_blueprint (Utilities|Casting|CastToUE4ASP_HeroTPP_AnimBlueprint (Components|SkeletalMesh|GetAnimInstance (Variables|Character|GetMesh))))
      (Variables|Default|SetAnimInstance _asue4asp_hero_tpp_anim_blueprint)
      (Development|PrintString "anim Instance has been set" true true "(R=0.044678,G=1.000000,B=0.000000,A=1.000000)"))
    (:then_1
      (if (Pawn|IsLocallyControlled)
        (Utilities|FlowControl|Sequence
          (:then_0
            (bind _returnvalue (UserInterface|CreateWidget "/Game/UI/WPB_Crroshair.WPB_Crroshair_C"))
            (UserInterface|Viewport|AddtoViewport _returnvalue 0))
          (:then_1
            (bind _returnvalue_2 (UserInterface|CreateWidget "/Game/UI/WBP_HealthIndicator.WBP_HealthIndicator_C"))
            (UserInterface|Viewport|AddtoViewport _returnvalue_2 0)))))))

(event Input|ActionEvents|InputActionZoom
  (params (Key :type Key%20Structure))
  (:Pressed
    (bind _zoom (Timeline|Zoom Play)
      (:Update
        (Camera|SetFieldOfView (Variables|Default|GetCameraComp) _zoom))))
  (:Released
    (Utilities|String|Reverse (Variables|Default|GetZoom))))

(event Input|MouseEvents|LeftMouseButton
  (params (Key :type Key%20Structure))
  ;[1 1 1] For Testing purpose only
  (:Pressed
    (Utilities|Time|SetGlobalTimeDilation 0.1))
  (:Released
    (Utilities|Time|SetGlobalTimeDilation 1.0)))

(event Input|KeyboardEvents|E
  (params (Key :type Key%20Structure))
  ;[1 1 1] For Testing purpose only
  (:Pressed
    (bind _output_get (Variables|Default|SetIKTraceDistance (+ (Variables|Default|GetIKTraceDistance) 1e+01)))
    (Development|PrintString (Utilities|String|ToString(Float) _output_get))))

(event Input|KeyboardEvents|Q
  (params (Key :type Key%20Structure))
  ;[1 1 1] For Testing purpose only
  (:Pressed
    (bind _output_get (Variables|Default|SetIKTraceDistance (+ (Variables|Default|GetIKTraceDistance) -1e+01)))
    (Development|PrintString (Utilities|String|ToString(Float) _output_get))))

(event Input|KeyboardEvents|R
  (params (Key :type Key%20Structure))
  ;[1 1 1] For Testing purpose only
  (:Pressed
    (Utilities|FlowControl|FlipFlop
      (:A
        (Variables|Default|SetIKOptimization true))
      (:B
        (Variables|Default|SetIKOptimization false)))
    (Development|PrintString (Utilities|String|ToString(Boolean) (Variables|Default|GetIKOptimization)))))

(fn ConstructionScript
  ;[1 1 1] Get Capsule Half Height
  (Variables|Default|SetIKCapsuleHalfHeight (Components|Capsule|GetScaledCapsuleHalfHeight (Variables|Default|GetCapsuleComponent))))

(fn NormaltoRotator
  (params (Normal :type Vector))
  (bind (_x _y _z) (Math|Vector|BreakVector Normal))
  ;[1 1 1] A pure Function to convert Normal to Rotation
  (return (Math|Rotator|MakeRotator (Class|KismetMathLibrary|DegAtan2 _y _z) (* (Class|KismetMathLibrary|DegAtan2 _x _z) -1.0) 0.0)))

(fn IKUpdateFootOffset
  (params (TargetValue :type Float%20%28single-precision%29) (EffectorVar :type Float%20%28single-precision%29) (InterpSpeed :type Float%20%28single-precision%29))
  ;[1 1 1] Tick pass-by-refference tick box in the input options  for Effector Var
  (LocalVariables|SetTarget TargetValue)
  ;[1 1 1] Setting the value of effect using pass by reffereance
  (|SetBy-RefVar EffectorVar (Math|Interpolation|FInterpTo EffectorVar (LocalVariables|GetTarget) (Variables|Default|GetDeltaSeconds) InterpSpeed)))

(fn IKUpdateFootRotation
  (params (TargetValue :type Rotator) (RotationVar :type Rotator) (InterpSpeed :type Float%20%28single-precision%29))
  ;[1 1 1] Updating foot rotation
  (LocalVariables|SetTarget TargetValue)
  (|SetBy-RefVar RotationVar (Math|Interpolation|RInterpTo RotationVar (LocalVariables|GetTarget) (Variables|Default|GetDeltaSeconds) InterpSpeed)))

(fn UpdateCApsuleHalfHeight
  (params (HipsShifts :type Float%20%28single-precision%29) (Reset%20Default :type Boolean))
  (bind _capsulecomponent (Variables|Default|GetCapsuleComponent))
  (Components|Capsule|SetCapsuleHalfHeight _capsulecomponent (Math|Interpolation|FInterpTo (Components|Capsule|GetScaledCapsuleHalfHeight _capsulecomponent) (Math|Float|SelectFloat (Variables|Default|GetIKCapsuleHalfHeight) (- (Variables|Default|GetIKCapsuleHalfHeight) (/ (Math|Float|Absolute(Float) HipsShifts) 2.0)) Reset%20Default) (Variables|Default|GetDeltaSeconds) (Variables|Default|GetIKHipsInterpSpeed)) true))

(fn IKResetVars
  (bind _animinstance (Variables|Default|GetAnimInstance))
  (bind _ikfeetinterpspeed (Variables|Default|GetIKFeetInterpSpeed))
  (bind _animinstance_2 (Variables|Default|GetAnimInstance))
  (bind _ikfeetinterpspeed_2 (Variables|Default|GetIKFeetInterpSpeed))
  (Utilities|FlowControl|Sequence
    (:then_0
      ;[1 1 1] To smoothly  reset the default values when character begin to move
      (CallFunction|IKUpdateFootOffset 0.0 (Variables|/Game/AnimStarterPack/UE4ASP_HeroTPP_AnimBlueprint.UE4ASP_HeroTPP_AnimBlueprint_C|GetRightEffecorLoc _animinstance) _ikfeetinterpspeed)
      (CallFunction|IKUpdateFootOffset 0.0 (Variables|/Game/AnimStarterPack/UE4ASP_HeroTPP_AnimBlueprint.UE4ASP_HeroTPP_AnimBlueprint_C|GetLeftEffectorLoc _animinstance) _ikfeetinterpspeed))
    (:then_1
      (CallFunction|IKUpdateFootRotation "0, 0, 0" (Variables|/Game/AnimStarterPack/UE4ASP_HeroTPP_AnimBlueprint.UE4ASP_HeroTPP_AnimBlueprint_C|GetRightFootRotation _animinstance_2) _ikfeetinterpspeed_2)
      (CallFunction|IKUpdateFootRotation "0, 0, 0" (Variables|/Game/AnimStarterPack/UE4ASP_HeroTPP_AnimBlueprint.UE4ASP_HeroTPP_AnimBlueprint_C|GetLeftFootRotation _animinstance_2) _ikfeetinterpspeed_2))
    (:then_2
      (CallFunction|IKUpdateFootOffset 0.0 (Variables|/Game/AnimStarterPack/UE4ASP_HeroTPP_AnimBlueprint.UE4ASP_HeroTPP_AnimBlueprint_C|GetHipsOffset (Variables|Default|GetAnimInstance)) (Variables|Default|GetIKHipsInterpSpeed))
      (CallFunction|UpdateCApsuleHalfHeight 0.0 false))))

(fn IsMoving
  ;[1 1 1] This is a pure function
  (return (> (Math|Vector|VectorLength (Transformation|GetVelocity)) 0.0)))

(fn IKupdate
  (Utilities|FlowControl|Sequence
    (:then_0
      ;[1 1 1] Calulate foot offset and rotation
      (bind (_offest _impact) (CallFunction|IKFootTrace (Variables|Default|GetIKTraceDistance) (Variables|Default|GetIKLeftSocket)))
      (LocalVariables|SetLEftFootOffset _offest)
      (CallFunction|IKUpdateFootRotation (CallFunction|NormaltoRotator _impact) (Variables|/Game/AnimStarterPack/UE4ASP_HeroTPP_AnimBlueprint.UE4ASP_HeroTPP_AnimBlueprint_C|GetLeftFootRotation (Variables|Default|GetAnimInstance)) (Variables|Default|GetIKFeetInterpSpeed)))
    (:then_1
      (bind (_offest_2 _impact_2) (CallFunction|IKFootTrace (Variables|Default|GetIKTraceDistance) (Variables|Default|GetIKRightSocket)))
      (LocalVariables|SetRightFootOffset _offest_2)
      (CallFunction|IKUpdateFootRotation (CallFunction|NormaltoRotator _impact_2) (Variables|/Game/AnimStarterPack/UE4ASP_HeroTPP_AnimBlueprint.UE4ASP_HeroTPP_AnimBlueprint_C|GetRightFootRotation (Variables|Default|GetAnimInstance)) (Variables|Default|GetIKFeetInterpSpeed)))
    (:then_2
      ;[1 1 1] Update hip Translation
      (LocalVariables|SetHipsOffest (Math|Float|SelectFloat (Math|Float|Min(Float) (LocalVariables|GetLEftFootOffset) (LocalVariables|GetRightFootOffset)) 0.0 (< (Math|Float|Min(Float) (LocalVariables|GetLEftFootOffset) (LocalVariables|GetRightFootOffset)) 0.0)))
      (CallFunction|IKUpdateFootOffset (Math|Float|SelectFloat (Math|Float|Min(Float) (LocalVariables|GetLEftFootOffset) (LocalVariables|GetRightFootOffset)) 0.0 (< (Math|Float|Min(Float) (LocalVariables|GetLEftFootOffset) (LocalVariables|GetRightFootOffset)) 0.0)) (Variables|/Game/AnimStarterPack/UE4ASP_HeroTPP_AnimBlueprint.UE4ASP_HeroTPP_AnimBlueprint_C|GetHipsOffset (Variables|Default|GetAnimInstance)) (Variables|Default|GetIKHipsInterpSpeed))
      ;[1 1 1] Update Capsule Height with the new hip offset
      (CallFunction|UpdateCApsuleHalfHeight (LocalVariables|GetHipsOffest) false))
    (:then_3
      ;[1 1 1] Update effector locations of both feet
      (CallFunction|IKUpdateFootOffset (- (LocalVariables|GetLEftFootOffset) (LocalVariables|GetHipsOffest)) (Variables|/Game/AnimStarterPack/UE4ASP_HeroTPP_AnimBlueprint.UE4ASP_HeroTPP_AnimBlueprint_C|GetLeftEffectorLoc (Variables|Default|GetAnimInstance)) (Variables|Default|GetIKFeetInterpSpeed))
      (CallFunction|IKUpdateFootOffset (- (LocalVariables|GetRightFootOffset) (LocalVariables|GetHipsOffest)) (Variables|/Game/AnimStarterPack/UE4ASP_HeroTPP_AnimBlueprint.UE4ASP_HeroTPP_AnimBlueprint_C|GetRightEffecorLoc (Variables|Default|GetAnimInstance)) (Variables|Default|GetIKFeetInterpSpeed)))
    (:then_4
      ;[1 1 1] To disable IK when we get the desired state
      (if (and (Math|Float|NearlyEqual(Float) (Variables|/Game/AnimStarterPack/UE4ASP_HeroTPP_AnimBlueprint.UE4ASP_HeroTPP_AnimBlueprint_C|GetLeftEffectorLoc (Variables|Default|GetAnimInstance)) (- (LocalVariables|GetLEftFootOffset) (LocalVariables|GetHipsOffest)) 1.0) (Math|Float|NearlyEqual(Float) (Variables|/Game/AnimStarterPack/UE4ASP_HeroTPP_AnimBlueprint.UE4ASP_HeroTPP_AnimBlueprint_C|GetRightEffecorLoc (Variables|Default|GetAnimInstance)) (- (LocalVariables|GetRightFootOffset) (LocalVariables|GetHipsOffest)) 1.0))
        (CallFunction|DisableIK)))))

(fn IKFootTrace
  (params (TraceDistance :type Float%20%28single-precision%29) (SocketName :type Name))
  (bind _returnvalue (Transformation|GetActorLocation))
  (bind _z (Math|Vector|BreakVector _returnvalue))
  ;[1 1 1] Storing to local Variable
  (LocalVariables|SetDistance TraceDistance)
  (LocalVariables|SetSocket SocketName)
  (bind _outhit (Collision|LineTraceByChannel (Math|Vector|MakeVector (.X (Math|Vector|BreakVector (Transformation|GetSocketLocation (Variables|Character|GetMesh) (LocalVariables|GetSocket)))) (.Y (Math|Vector|BreakVector (Transformation|GetSocketLocation (Variables|Character|GetMesh) (LocalVariables|GetSocket)))) _z) (Math|Vector|MakeVector (.X (Math|Vector|BreakVector (Transformation|GetSocketLocation (Variables|Character|GetMesh) (LocalVariables|GetSocket)))) (.Y (Math|Vector|BreakVector (Transformation|GetSocketLocation (Variables|Character|GetMesh) (LocalVariables|GetSocket)))) (- (- _z (Variables|Default|GetIKCapsuleHalfHeight)) (LocalVariables|GetDistance))) "TraceTypeQuery1" true 0 "None"))
  (LocalVariables|SetValidHit (.bblockinghit _outhit))
  (return (Math|Float|SelectFloat (+ (Variables|Default|GetIKAdjustOffset) (- (Math|Vector|VectorLength (- (.location _outhit) (.traceend _outhit))) (LocalVariables|GetDistance))) 0.0 (LocalVariables|GetValidHit)) (.normal _outhit)))

(event Input|KeyboardEvents|E
  (params (Key :type Key%20Structure))
  (:Pressed
    (Utilities|FlowControl|FlipFlop)))

(event Custom|DisableIK
  (Utilities|FlowControl|Delay (Variables|Default|GetIKTimeout))
  (Utilities|FlowControl|Gate true) ; enters at Close
)

(event Custom|EnableIK
  (Utilities|FlowControl|Gate true) ; enters at Open
)